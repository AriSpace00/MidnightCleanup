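; BP_TruckInCollision is an overlap actor that tracks whether the player is inside the truck.
; On begin overlap with a PlayerCharacter controlled by a PC, it sets the controller's IsInTruck flag, activates the character's Trace3DWidget and enables its hit testing.
; End overlap clears the flag, deactivates the component and disables hit testing, so this 3D widget tracing is switched on only while inside.
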(event `self.ReceiveActorBeginOverlap`
  (params (OtherActor :type "Actor Object Reference"))
  (bind _asplayer_character (cast `PlayerCharacter` OtherActor))
  (bind _aspc (cast `PC` (`Pawn.GetController` _asplayer_character)))
  (set `PC.bIsInTruck` true _aspc)
  (bind _trace3dwidget (`PlayerCharacter.Trace3DWidget` _asplayer_character))
  (`ActorComponent.Activate` _trace3dwidget false)
  (set `WidgetInteractionComponent.bEnableHitTesting` true _trace3dwidget))

(event `self.ReceiveActorEndOverlap`
  (params (OtherActor :type "Actor Object Reference"))
  (bind _asplayer_character (cast `PlayerCharacter` OtherActor))
  (bind _aspc (cast `PC` (`Pawn.GetController` _asplayer_character)))
  (set `PC.bIsInTruck` false _aspc)
  (bind _trace3dwidget (`PlayerCharacter.Trace3DWidget` _asplayer_character))
  (`ActorComponent.Deactivate` _trace3dwidget)
  (set `WidgetInteractionComponent.bEnableHitTesting` false _trace3dwidget))

(fn `UserConstructionScript`)
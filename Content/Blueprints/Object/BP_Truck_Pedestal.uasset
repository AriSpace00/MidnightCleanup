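; BP_Truck_Pedestal is a truck pedestal actor that animates when its FinishPlay event is called.
; After a short delay, a timeline drives the Pedestal component's relative roll.
; Whenever that rotation value equals exactly zero during an update, it plays a second timeline, 들어가기 ("going in"), which sets the StaticMesh's world Y while keeping X and Z.
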(event `self.ReceiveBeginPlay`)

(event `FinishPlay`
  (bind (_returnvalue_x _returnvalue_y _returnvalue_z) (`KismetMathLibrary.BreakVector` (`SceneComponent.K2_GetComponentLocation` (`self.StaticMesh`))))
  (`KismetSystemLibrary.Delay` 2.0)
  (bind (_direction _rotate) (`Timeline|타임라인`)
    (:`Update`
      (`SceneComponent.K2_SetRelativeRotation` (`self.Pedestal`) (`KismetMathLibrary.MakeRotator` _rotate) false false)
      (if (== _rotate 0.0)
        (bind (_direction_2 `_새_트랙_0`) (`Timeline|들어가기`)
          (:`Update`
            (`SceneComponent.K2_SetWorldLocation` (`self.StaticMesh`) (`KismetMathLibrary.MakeVector` _returnvalue_x `_새_트랙_0` _returnvalue_z) false false)))))))

(fn `UserConstructionScript`)
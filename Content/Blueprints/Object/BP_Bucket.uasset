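; Bucket object that shows a water surface when filled and exposes events to control two Niagara effects, a general one and a spoil one.
; Both effects start deactivated with force solo on; the general effect can be enabled, disabled or given a new system, while the spoil effect only has an enable event.
; Tick syncs water plane visibility to IsFilled and keeps it level in world space, following only the bucket's yaw.
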(event `self.EnableEffect`
  ;[0 0.1725 1] Enable Effect
  (`ActorComponent.Activate` (`self.Niagara`) false))

(event `self.EnableSpoilEffect`
  ;[0 0.1725 1] Enable Effect
  (`ActorComponent.Activate` (`self.Spoil`) false))

(event `self.ReceiveBeginPlay`
  ;[1 1 1] BeginPlay
  (`ActorComponent.Deactivate` (`self.Niagara`))
  (`ActorComponent.Deactivate` (`self.Spoil`))
  (`NiagaraComponent.SetForceSolo` (`self.Niagara`) true)
  (`NiagaraComponent.SetForceSolo` (`self.Spoil`) true))

(event `self.DisableEffect`
  ;[0 0.1725 1] Disable Effect
  (`ActorComponent.Deactivate` (`self.Niagara`)))

(event `self.SetEffect`
  (params (NiagaraSystem :type "NiagaraSystem Object Reference"))
  ;[0 0.1725 1] Set Effect
  (`NiagaraComponent.SetAsset` (`self.Niagara`) NiagaraSystem true))

(event `self.ReceiveTick`
  (params (DeltaSeconds :type "Float (single-precision)"))
  (bind (_returnvalue_roll _returnvalue_pitch _returnvalue_yaw) (`KismetMathLibrary.BreakRotator` (`self.K2_GetActorRotation`)))
  ;[1 1 1] Tick
  (`SceneComponent.SetVisibility` (`self.WaterPlane`) (`self.bIsFilled`) false)
  (`SceneComponent.K2_SetWorldRotation` (`self.WaterPlane`) (`KismetMathLibrary.MakeRotator` 0.0 180.0 _returnvalue_yaw) false false))

(fn `UserConstructionScript`)
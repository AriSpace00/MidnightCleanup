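; BP_TrashIndicator is an indicator Blueprint whose widget component appears when the player is holding a box or trash.
; ShowIndicator checks the given player's held state, then makes the widget visible and plays the WBP_TrashIndicator fade-in.
; HideIndicator plays the fade-out and waits for the duration the widget reports before hiding it.
; CheckIndicator toggles visibility directly from a boolean, without animation.
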(event `self.CheckIndicator`
  (params (State :type Boolean))
  (if State
    (`SceneComponent.SetVisibility` (`self.Widget`) true false)
    (else
      (`SceneComponent.SetVisibility` (`self.Widget`) false false))))

(event `self.HideIndicator`
  (bind _aswbp_trash_indicator (cast `/Game/UI/Indicator/WBP_TrashIndicator` (`WidgetComponent.GetWidget` (`self.Widget`))))
  (`/Game/UI/Indicator/WBP_TrashIndicator.PlayFadeOutAnim` _aswbp_trash_indicator)
  (bind _duration (`/Game/UI/Indicator/WBP_TrashIndicator.GetDuration` _aswbp_trash_indicator))
  (`KismetSystemLibrary.Delay` _duration)
  (`SceneComponent.SetVisibility` (`self.Widget`) false false))

(event `self.ShowIndicator`
  (params (InPlayer :type "PlayerCharacter Object Reference"))
  (`/Engine/EditorBlueprintResources/StandardMacros.IsValid` InPlayer
    (:`Is Valid`
      (if (or (`PlayerCharacter.bIsHeldBox` InPlayer) (`PlayerCharacter.bIsHeldTrash` InPlayer))
        (`SceneComponent.SetVisibility` (`self.Widget`) true false)
        (bind _aswbp_trash_indicator (cast `/Game/UI/Indicator/WBP_TrashIndicator` (`WidgetComponent.GetWidget` (`self.Widget`))))
        (`/Game/UI/Indicator/WBP_TrashIndicator.PlayFadeInAnim` _aswbp_trash_indicator)))))

(fn `UserConstructionScript`)
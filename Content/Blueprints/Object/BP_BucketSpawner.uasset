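; BP_BucketSpawner is a bucket spawner object that shows twelve static meshes according to CurrentObjectNum; the file contains no spawning logic.
; Every Tick it unhides all meshes, then hides the first CurrentObjectNum in a fixed, non-sequential order, so fewer remain visible as the count rises.
; A switch, with every case feeding one shared loop, limits hiding to counts of one through twelve.
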(event `self.ReceiveTick`
  (params (DeltaSeconds :type "Float (single-precision)"))
  (bind _array (`|MakeArray` (`self.StaticMesh3`) (`self.StaticMesh6`) (`self.StaticMesh2`) (`self.StaticMesh4`) (`self.StaticMesh5`) (`self.StaticMesh1`) (`self.StaticMesh9`) (`self.StaticMesh10`) (`self.StaticMesh7`) (`self.StaticMesh8`) (`self.StaticMesh12`) (`self.StaticMesh11`)))
  (bind _returnvalue (- (`self.CurrentObjectNum`) 1))
  (`SceneComponent.SetHiddenInGame` _array false false)
  (switch `int` _returnvalue
    (:`0`
      _)
    (:`1`
      _)
    (:`2`
      _)
    (:`3`
      _)
    (:`4`
      _)
    (:`5`
      _)
    (:`6`
      _)
    (:`7`
      _)
    (:`8`
      _)
    (:`9`
      _)
    (:`10`
      _)
    (:`11`
      _))
  (for _index (range (+ _returnvalue 1))
    (`SceneComponent.SetHiddenInGame` (`|GetArrayItem` _array _index) true false)))

(fn `UserConstructionScript`)
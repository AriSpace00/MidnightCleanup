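; BP_TruckDoor_R is a right-side truck door that swings with sound during the game's opening and again when FinishPlay is called.
; BeginPlay waits OpeningTime, timed to the opening subtitles, then plays the AudioCurveSource and a timeline that drives the static mesh's world yaw.
; FinishPlay replays the sound and rotates the mesh through a second timeline, with no delay.
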(event `self.ReceiveBeginPlay`
  (`KismetSystemLibrary.Delay` (`self.OpeningTime`)) ; 오프닝 자막 시간만큼 딜레이
  (`AudioComponent.Play` (`self.AudioCurveSource`) 0.0)
  (bind (_direction _rotate) (`Timeline|타임라인`)
    (:`Update`
      (`SceneComponent.K2_SetWorldRotation` (`self.StaticMesh`) (`KismetMathLibrary.MakeRotator` 0.0 0.0 _rotate) false false))))

(event `FinishPlay`
  (`AudioComponent.Play` (`self.AudioCurveSource`) 0.0)
  (bind (_direction _rotate) (`Timeline|타임라인_0`)
    (:`Update`
      (`SceneComponent.K2_SetWorldRotation` (`self.StaticMesh`) (`KismetMathLibrary.MakeRotator` 0.0 0.0 _rotate) false false))))

(fn `UserConstructionScript`)
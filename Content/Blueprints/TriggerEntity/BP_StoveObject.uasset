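; BP_StoveObject is a stove prop whose smoke and fire effects can be switched on and off.
; On BeginPlay it deactivates both effect components and sets Force Solo on them, so each simulates as its own instance.
; The custom events EnableEffect and DisableEffect activate or deactivate both effects together and print a debug string.
; Nothing in this Blueprint calls these events.
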(event `self.ReceiveBeginPlay`
  ;[1 1 1] BeginPlay
  (`ActorComponent.Deactivate` (`self.Smoke`))
  (`ActorComponent.Deactivate` (`self.Fire`))
  (`NiagaraComponent.SetForceSolo` (`self.Smoke`) true)
  (`NiagaraComponent.SetForceSolo` (`self.Fire`) true))

(event `self.EnableEffect`
  ;[0 0.1725 1] Enable Effect
  (`ActorComponent.Activate` (`self.Smoke`) false)
  (`ActorComponent.Activate` (`self.Fire`) false)
  (`KismetSystemLibrary.PrintString` "SpawnEffect"))

(event `self.DisableEffect`
  ;[0 0.1725 1] Disable Effect
  (`ActorComponent.Deactivate` (`self.Smoke`))
  (`ActorComponent.Deactivate` (`self.Fire`))
  (`KismetSystemLibrary.PrintString` "DestroyEffect"))

(fn `UserConstructionScript`)
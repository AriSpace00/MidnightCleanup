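; A trigger actor that shows a one-time notification caption when players enter the wooden plank disposal area.
; Box overlap records each unique PlayerCharacter and requests the caption unless the PrimaryWoodenPlankDisposalArea flag on its BP_InGamePC is already set.
; That flag is set after the request only when EnableCaption is false on the controller.
; Tick destroys the actor once the recorded count reaches the GameState player count.
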(event `self.Box.OnComponentBeginOverlap`
  (params (OverlappedComponent :type "PrimitiveComponent Object Reference") (OtherActor :type "Actor Object Reference") (OtherComp :type "PrimitiveComponent Object Reference") (OtherBodyIndex :type Integer) (bFromSweep :type Boolean) (SweepResult :type "HitResult Structure (by ref)"))
  (if (> (`KismetArrayLibrary.Array_Length` (`GameStateBase.PlayerArray` (`GameplayStatics.GetGameState`))) (`KismetArrayLibrary.Array_Length` (`self.OverlappedPlayers_WoodenPlankDisposal`)))
    (bind _asplayer_character (cast `PlayerCharacter` OtherActor))
    (if (< (`KismetArrayLibrary.Array_Find` (`self.OverlappedPlayers_WoodenPlankDisposal`) _asplayer_character) 0)
      (`KismetArrayLibrary.Array_Add` (`self.OverlappedPlayers_WoodenPlankDisposal`) _asplayer_character)
      (bind _asbp_in_game_pc (cast `/Game/Blueprints/Common/GameplayFramework/InGame/BP_InGamePC` (`Pawn.GetController` _asplayer_character)))
      (if (not (`PC.bPrimaryWoodenPlankDisposalArea` _asbp_in_game_pc))
        (`PlayerCharacter.UpdateCaptionByCollision` _asplayer_character "PrimaryNotify_WoodenPlankDisposalArea" 1.0)
        (if (not (`PC.bEnableCaption` _asbp_in_game_pc))
          (set `PC.bPrimaryWoodenPlankDisposalArea` true _asbp_in_game_pc))))))

(event `self.ReceiveTick`
  (params (DeltaSeconds :type "Float (single-precision)"))
  (if (>= (`KismetArrayLibrary.Array_Length` (`self.OverlappedPlayers_WoodenPlankDisposal`)) (`KismetArrayLibrary.Array_Length` (`GameStateBase.PlayerArray` (`GameplayStatics.GetGameState`))))
    (`self.K2_DestroyActor`)))

(fn `UserConstructionScript`)
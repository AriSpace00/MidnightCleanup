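; BP_Axe is an axe tool actor that carries a switchable Niagara effect.
; On BeginPlay it deactivates the Niagara component and sets it to force solo simulation.
; Custom events activate or deactivate the effect, or swap its Niagara system asset while resetting existing override parameters.
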(event `self.ReceiveBeginPlay`
  ;[1 1 1] BeginPlay
  (`ActorComponent.Deactivate` (`self.Niagara`))
  (`NiagaraComponent.SetForceSolo` (`self.Niagara`) true))

(event `self.EnableEffect`
  ;[0 0.1725 1] Enable Effect
  (`ActorComponent.Activate` (`self.Niagara`) false))

(event `self.DisableEffect`
  ;[0 0.1725 1] Disable Effect
  (`ActorComponent.Deactivate` (`self.Niagara`)))

(event `self.SetEffect`
  (params (NiagaraSystem :type "NiagaraSystem Object Reference"))
  ;[0 0.1725 1] Set Effect
  (`NiagaraComponent.SetAsset` (`self.Niagara`) NiagaraSystem true))

(fn `UserConstructionScript`)
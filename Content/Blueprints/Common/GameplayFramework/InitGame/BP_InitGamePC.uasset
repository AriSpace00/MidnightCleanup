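; BP_InitGamePC, apparently the init-game player controller, holds an unfinished F1 debug hook for setting the player's name.
; F1 calls a custom event that invokes S2ASetName.
; The s2A_SetName event casts player state 0 and the game instance, then calls GetUserID without using the result.
; The logic writing that ID to BP_InGamePS.UserName is disconnected and never runs.
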(event `self.ReceiveTick`
  (params (DeltaSeconds :type "Float (single-precision)")))

(event `Key|F1`
  (params (Key :type "Key Structure"))
  (:`Pressed`
    (`self.새 함수`)))

(event `새 함수`
  (`self.s2A_SetName`))

(event `s2A_SetName`
  (cast `/Game/Blueprints/Common/GameplayFramework/InGame/BP_InGamePS` (`GameplayStatics.GetPlayerState` 0))
  (bind _asbp_gi (cast `/Game/Blueprints/Common/BP_GI` (`GameplayStatics.GetGameInstance`)))
  (`GI.GetUserID` _asbp_gi))

(fn `UserConstructionScript`)
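; BP_InGameGS_3p is the in-game 3p gameplay framework Blueprint, likely a GameState, that runs the end-of-game sequence.
; EndGame looks up the out-truck cine camera and both truck doors by class and calls FinishPlay on each.
; Timed delays then stage the truck pedestal's FinishPlay, the finish widget and finally the reward widget.
; BeginPlay, Tick and the construction script are empty.
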(event `self.EndGame`
  (bind _returnvalue (`GameplayStatics.GetActorOfClass` "/Game/Blueprints/BP_OutTruckCineCamera.BP_OutTruckCineCamera_C"))
  (`/Game/Blueprints/BP_OutTruckCineCamera.Finish play` _returnvalue)
  (bind _returnvalue_2 (`GameplayStatics.GetActorOfClass` "/Game/Blueprints/Object/BP_TruckDoor_L.BP_TruckDoor_L_C"))
  (`/Game/Blueprints/Object/BP_TruckDoor_L.FinishPlay` _returnvalue_2)
  (bind _returnvalue_3 (`GameplayStatics.GetActorOfClass` "/Game/Blueprints/Object/BP_TruckDoor_R.BP_TruckDoor_R_C"))
  (`/Game/Blueprints/Object/BP_TruckDoor_R.FinishPlay` _returnvalue_3)
  (`KismetSystemLibrary.Delay` 2.0)
  (bind _returnvalue_4 (`GameplayStatics.GetActorOfClass` "/Game/Blueprints/Object/BP_Truck_Pedestal.BP_Truck_Pedestal_C"))
  (`/Game/Blueprints/Object/BP_Truck_Pedestal.FinishPlay` _returnvalue_4)
  (`KismetSystemLibrary.Delay` 7.0)
  (`self.ShowFinishWidget`)
  (`KismetSystemLibrary.Delay` 3.0)
  (`self.ShowRewardWidget`))

(fn `UserConstructionScript`)
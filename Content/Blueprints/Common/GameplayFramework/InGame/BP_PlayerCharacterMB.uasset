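; In-game player character Blueprint that gates player input during the tutorial and moves the camera to a computer.
; On BeginPlay it disables input for the tutorial time read from the game state, then re-enables it.
; MoveCameratoComputer locks input while a timeline slides the camera along a given spline, then enables the laptop and restores input.
; S2C events toggle input only when the local controller possesses this pawn.
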(event `S2C_EnableInput`
  (`/Engine/EditorBlueprintResources/StandardMacros.IsValid` (`GameplayStatics.GetPlayerController` 0)
    (:`Is Valid`
      (if (== (`Controller.K2_GetPawn` (`GameplayStatics.GetPlayerController` 0)) self)
        (`self.EnableInput` (`GameplayStatics.GetPlayerController` 0))))))

(event `S2C_DisableInput`
  (`/Engine/EditorBlueprintResources/StandardMacros.IsValid` (`GameplayStatics.GetPlayerController` 0)
    (:`Is Valid`
      (if (== (`Controller.K2_GetPawn` (`GameplayStatics.GetPlayerController` 0)) self)
        (`self.DisableInput` (`GameplayStatics.GetPlayerController` 0))))))

(event `self.ReceiveBeginPlay`
  (bind _aspc (cast `PC` (`GameplayStatics.GetPlayerController` 0)))
  (`/Engine/EditorBlueprintResources/StandardMacros.IsValid` _aspc
    (:`Is Valid`
      (`self.S2C_DisableInput`)
      (bind _asin_game_gs (cast `InGameGS` (`GameplayStatics.GetGameState`)))
      (`KismetSystemLibrary.Delay` (`KismetMathLibrary.Conv_IntToDouble` (`InGameGS.TutorialTime` _asin_game_gs)))
      (`self.S2C_EnableInput`))))

(event `self.MoveCameraToComputer`
  (params (InPath :type "SplineComponent Object Reference"))
  (`self.S2C_DisableInput`)
  (bind (_direction _duration) (`Timeline|타임라인` :!via `PlayFromStart`)
    (:`Update`
      (`self.SetCameraLocation` (`SplineComponent.GetLocationAtDistanceAlongSpline` InPath (* _duration (`SplineComponent.GetSplineLength` InPath)) "World")))
    (:`Finished`
      (`self.EnableLaptop`)
      (`self.S2C_EnableInput`))))

(fn `UserConstructionScript`)
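; BP_TruckSound is an actor that delays a truck sound until the tutorial period of the match has passed.
; On BeginPlay it deactivates its Audio component, reads TutorialTime from the InGameGS game state and prints it for debugging.
; After waiting that long, it activates the audio again; if the game state cast fails, the sound stays off.
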(event `self.ReceiveBeginPlay`
  (`ActorComponent.Deactivate` (`self.Audio`))
  (bind _asin_game_gs (cast `InGameGS` (`GameplayStatics.GetGameState`)))
  (bind _tutorialtime (`InGameGS.TutorialTime` _asin_game_gs))
  (`KismetSystemLibrary.PrintString` (`KismetStringLibrary.Conv_IntToString` _tutorialtime))
  (`KismetSystemLibrary.Delay` (`KismetMathLibrary.Conv_IntToDouble` _tutorialtime))
  (`ActorComponent.Activate` (`self.Audio`) false))

(fn `UserConstructionScript`)
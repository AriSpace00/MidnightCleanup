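; Water effect actor for an angled breach splash, built from a main mesh and a mist mesh that play on BeginPlay with Autoplay or via SpawnSplash.
; A timeline animates phase, opacity, refraction and mask material parameters, scaled by tunable variables.
; A longer ripple timeline only times optional actor destruction, as ripple, whitewater and audio logic are disconnected.
; The construction script clears the mesh of disabled layers.
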(event `self.ReceiveBeginPlay`
  (bind _mist_mesh (`self.Mist_mesh`))
  (bind _main_mesh (`self.Main_mesh`))
  (bind _array (`|MakeArray` (`self.Main_mesh`) (`self.Mist_mesh`) :!type "SceneComponent Object Reference"))
  ;[0 1 0.0718] Good for Spawning
  (`|ExecutionSequence`
    (:`then_0`
      ;[1 1 1] Initalize
      (set `self.CustomTimeDilation` (`self.Speed`))
      (`SceneComponent.SetHiddenInGame` _array true false))
    (:`then_1`
      (if (`self.Autoplay`)
        (`SceneComponent.SetHiddenInGame` _array false false :!label _label)
        (`|ExecutionSequence`
          (:`then_0`
            (bind (_direction _zero_to_one_linear__shared_ _ior__shared_ _opacitymasksize__main_ _refractmasksize__main_ _opacity__main_ _opacity__mist_ _opacity__ww_) (`Timeline|4_16 seconds` :`NewTime` (`self.CustomTimeDilation`) :!via `PlayFromStart`)
              (:`Update`
                (`|ExecutionSequence`
                  (:`then_0`
                    ;[1 1 1] Main
                    (`|ExecutionSequence`
                      (:`then_0`
                        (`MeshComponent.SetScalarParameterValueOnMaterials` _main_mesh "phase" (* _zero_to_one_linear__shared_ (`self.Phase_2Total`))))
                      (:`then_1`
                        (`MeshComponent.SetScalarParameterValueOnMaterials` _main_mesh "IOR" (+ (* _ior__shared_ (`self.IOR_add`)) 1.0)))
                      (:`then_2`
                        (`MeshComponent.SetScalarParameterValueOnMaterials` _main_mesh "OpacityMaskSize" (* _opacitymasksize__main_ (`self.OpacityMaskSize`))))
                      (:`then_3`
                        (`MeshComponent.SetScalarParameterValueOnMaterials` _main_mesh "Opacity" (* _opacity__main_ (`self.Main_Opacity`))))
                      (:`then_4`
                        (`MeshComponent.SetScalarParameterValueOnMaterials` _main_mesh "Refract_Mask_radius" (* _refractmasksize__main_ (`self.RefractMaskSize`))))))
                  (:`then_1`
                    ;[1 1 1] Mist
                    (`|ExecutionSequence`
                      (:`then_0`
                        (`MeshComponent.SetScalarParameterValueOnMaterials` _mist_mesh "phase" (* _zero_to_one_linear__shared_ (`self.Phase_2Total`))))
                      (:`then_1`
                        (`MeshComponent.SetScalarParameterValueOnMaterials` _mist_mesh "Opacity" (* _opacity__mist_ (`self.OpacityMist`))))))))
              (:`Finished`
                ;;[1 0.4062 0.4062] Destroy compents when finished (ripple will continue for a short time)
                (if (`self.AutoDestory`)
                  (`ActorComponent.K2_DestroyComponent` (`|MakeArray` (`self.Main_mesh`) (`self.Mist_mesh`) :!type "ActorComponent Object Reference"))))))
          (:`then_1`
            ;[1 1 1] Ripple
            (bind (_direction_2 _spike_and_drop _ease_out _opacity _ripple_height) (`Timeline|Ripple_5_4_Secs` :`NewTime` (`self.CustomTimeDilation`) :!via `PlayFromStart`)
              (:`Finished`
                ;[0.004132 0.1261 1] Destroy - Can be call here or in other BPs for optimization
                (`KismetSystemLibrary.Delay` 0.0)
                (if (`self.AutoDestory`)
                  (`self.K2_DestroyActor`))))))))))

(event `SpawnSplash`
  ;[0 1 0.06836] Input/Trigger here.  Good for custom setups (may want to turn off "Autoplay", and maybe the "AutoDestory" ).
  (goto _label))

(fn `UserConstructionScript`
  (`|ExecutionSequence`
    (:`then_1`
      (if (not (`self.Mist`))
        (`StaticMeshComponent.SetStaticMesh` (`self.Mist_mesh`) null)))
    (:`then_2`
      (if (not (`self.Main`))
        (`StaticMeshComponent.SetStaticMesh` (`self.Main_mesh`) null)))))